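; BP_Enemy is a sword-attacking enemy character that takes damage and ragdolls on death.
; AnyDamage lowers a stat in BPCStats; the health-bar hookup to its widget is left unconnected.
; SwordAttack plays a combo montage, while Begin/EndSwordTrace run a timed, debug-drawn sphere trace that calls ApplyDamage with no amount set, throttled by a resetting DoOnce.
; An unnamed custom event disables movement, enables mesh physics and sets IsDead, which stops tracing.
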(event `self.ReceiveBeginPlay`
  (bind _aswb_enemy_health (cast `/Game/UI/WB_EnemyHealth` (`WidgetComponent.GetWidget` (`self.Widget`)))))

(event `self.ReceiveAnyDamage`
  (params (Damage :type "Float (single-precision)") (DamageType :type "DamageType Object Reference") (InstigatedBy :type "Controller Object Reference") (DamageCauser :type "Actor Object Reference"))
  (`/Game/Blueprints/BPC_Stats.Increase Value` (`self.BPC_Stats`) "NewEnumerator0" (* Damage -1.0)))

(event `/Game/Blueprints/BPI_Damage.End Sword Trace`
  ;[0.05729 0.05729 0.05729 0.5] Sword Traces
  (if (`KismetSystemLibrary.K2_IsValidTimerHandle` (stale `/Game/Blueprints/BPI_Damage.Begin Sword Trace` _returnvalue))
    (`KismetSystemLibrary.K2_ClearAndInvalidateTimerHandle` (stale `/Game/Blueprints/BPI_Damage.Begin Sword Trace` _returnvalue))))

(event `/Game/Blueprints/BPI_Damage.Begin Sword Trace`
  ;[0.05729 0.05729 0.05729 0.5] Sword Traces
  (bind _returnvalue (`KismetSystemLibrary.K2_SetTimerDelegate` (delegate `Damage Trace`) 0.01)))

(event `Damage Trace`
  ;[0.05729 0.05729 0.05729 0.5] Sword Traces
  (if (not (`self.isDead?`))
    (bind (_outhit _returnvalue) (`KismetSystemLibrary.SphereTraceSingleForObjects` :`Start` (`SceneComponent.K2_GetComponentLocation` (`self.Start Dagger Trace Pos`)) :`End` (`SceneComponent.K2_GetComponentLocation` (`self.End Dagger Trace Pos`)) :`Radius` 100.0 :`ObjectTypes` (`|MakeArray` "ObjectTypeQuery3" :!type "EObjectTypeQuery Enum") :`DrawDebugType` "ForDuration" :`DrawTime` 3.0))
    (if _returnvalue
      (`/Engine/EditorBlueprintResources/StandardMacros.DoOnce` false :!label _label
        (:`Completed`
          (`GameplayStatics.ApplyDamage` (`.HitActor` (`GameplayStatics.BreakHitResult` _outhit)))
          (`KismetSystemLibrary.Delay` 0.3)
          (goto _label :!via `Reset`))))))

(event `CustomEvent`
  ;[0.05729 0.05729 0.05729 0.5] Die
  (`CharacterMovementComponent.DisableMovement` (`self.CharacterMovement`))
  (`PrimitiveComponent.SetSimulatePhysics` (`self.Mesh`) true)
  (set `self.isDead?` true))

(fn `Sword Attack`
  (returns (Duration :type "Float (double-precision)"))
  (bind _returnvalue (`self.PlayAnimMontage` "/Game/Characters/Souls/Combat/SwordAttackCombo_Montage.SwordAttackCombo_Montage"))
  (return _returnvalue))

(fn `UserConstructionScript`)