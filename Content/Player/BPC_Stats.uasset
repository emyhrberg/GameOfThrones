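; Player stats component that holds Health and Stamina, regenerates them and drives their progress bars.
; IncreaseValue clamps the chosen stat, updates its injected progress bar and, at zero health, sends DieMessage to the owner.
; A fast looping timer restores stamina while RegainStamina is set, plus health if the owning BP_ThirdPersonCharacter is alive.
; The separate RegainHealth timer runs an empty event.
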(event `self.ReceiveBeginPlay`
  ;[0.05729 0.05729 0.05729 0.5] Regain Stats
  (`KismetSystemLibrary.K2_SetTimerDelegate` (delegate `Regain Stamina`) 0.01 true)
  (`KismetSystemLibrary.K2_SetTimerDelegate` (delegate `Regain Health`) 0.01 true))

(event `Regain Stamina`
  ;[0.05729 0.05729 0.05729 0.5] Regain Stats
  (if (`self.regainStamina?`)
    (`self.Increase Value` "NewEnumerator1" 0.1)
    (bind _asbp_third_person_character (cast `/Game/Player/BP_ThirdPersonCharacter` (`self.GetOwner`)))
    (if (not (`/Game/Player/BP_ThirdPersonCharacter.isDead?` _asbp_third_person_character))
      (`self.Increase Value` "NewEnumerator0" 0.01))))

(event `Regain Health`
  ;[0.05729 0.05729 0.05729 0.5] Regain Stats
)

(event `Die`
  (message `/Game/Player/BPI_Damage.Die` (`self.GetOwner`)))

(event `Set Health Progress Bar`
  (params (`Health Progress Bar` :type "ProgressBar Object Reference"))
  (set `self.Health Progress Bar` `Health Progress Bar`))

(event `Set Stamina Progress Bar`
  (params (`Stamina Progress Bar` :type "ProgressBar Object Reference"))
  (set `self.Stamina Progress Bar` `Stamina Progress Bar`))

(fn `Increase Value`
  (params (Stat :type "/Game/Player/E_Stats Enum" :default "NewEnumerator0") (Value :type "Float (double-precision)"))
  (switch `/Game/Player/E_Stats` Stat
    (:`NewEnumerator0`
      ;[0.05729 0.05729 0.05729 0.5] Health
      (set `self.health` (`KismetMathLibrary.FClamp` (+ (`self.health`) Value) 0.0 (`self.maxHealth`)))
      (`|ExecutionSequence`
        (:`then_0`
          (if (<= (`self.health`) 0.0)
            (`self.Die`)))
        (:`then_1`
          (bind _health_progress_bar (`self.Health Progress Bar`)
            (:`then`
              (`ProgressBar.SetPercent` _health_progress_bar (/ (`self.health`) (`self.maxHealth`))))
            (:`else`)))))
    (:`NewEnumerator1`
      ;[0.05729 0.05729 0.05729 0.5] Stamina
      (set `self.stamina` (`KismetMathLibrary.FClamp` (+ (`self.stamina`) Value) 0.0 (`self.maxStamina`)))
      (bind _stamina_progress_bar (`self.Stamina Progress Bar`)
        (:`then`
          (`ProgressBar.SetPercent` _stamina_progress_bar (/ (`self.stamina`) (`self.maxStamina`))))
        (:`else`)))))