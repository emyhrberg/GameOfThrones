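; Player combat component for BP_ThirdPersonCharacter that handles target lock, dagger attacks and directional dodging, with stamina costs through BPCStats.
; Lock-on sphere-traces from the camera, attaches a marker actor and steers control rotation at the target until toggled off or the enemy dies.
; Montage notifies continue or stop the buffered combo, while timer-triggered sphere traces between dagger points apply damage.
; When locked on, the direction key selects the dodge montage.
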(event `self.ReceiveBeginPlay`
  ;[0.05729 0.05729 0.05729 0.5] Get Player Class
  (bind _asbp_third_person_character (cast `/Game/Player/BP_ThirdPersonCharacter` (`self.GetOwner`)))
  (set `self.Player BP` _asbp_third_person_character))

(event `EnhancedInput|/Game/Input/Actions/IA_Lock`
  (params (ActionValue :type Boolean) (ElapsedSeconds :type "Float (double-precision)") (TriggeredSeconds :type "Float (double-precision)") (InputAction :type "InputAction Object Reference" :default "/Game/Input/Actions/IA_Lock.IA_Lock"))
  (bind _returnvalue (`Actor.GetTransform` (`self.Target Lock Actor`)))
  (bind _transformcomponent (`PlayerCameraManager.TransformComponent` (`GameplayStatics.GetPlayerCameraManager` 0)))
  (bind _charactermovement (`Character.CharacterMovement` (`self.Player BP`)))
  (bind _charactermovement_2 (`Character.CharacterMovement` (`self.Player BP`)))
  (bind (_returnvalue_x _returnvalue_y _returnvalue_z) (`KismetMathLibrary.BreakVector` (`SceneComponent.K2_GetComponentLocation` _transformcomponent)))
  (bind _returnvalue_2 (`KismetMathLibrary.MakeVector` _returnvalue_x _returnvalue_y (+ _returnvalue_z 20.0)))
  ;[0.05729 0.05729 0.05729 0.5] Target Lock
  (:`Started`
    (`self.Target Lock Actor`
      (:`then`
        ;;[0.05729 0.05729 0.05729 0.5] Target Lock Off
        (`KismetSystemLibrary.PrintString` "target lock off")
        (set `self.isTargetLocked?` false)
        (set `self.movementDirection` "NewEnumerator0")
        (set `self.Target Lock Actor` null)
        (set `CharacterMovementComponent.bOrientRotationToMovement` true _charactermovement)
        (set `CharacterMovementComponent.bUseControllerDesiredRotation` false _charactermovement)
        (`Actor.K2_DestroyActor` (`self.Target Lock Widget`)))
      (:`else`
        (`KismetSystemLibrary.PrintString` "target lock on")
        (bind (_outhit _returnvalue_3) (`KismetSystemLibrary.SphereTraceSingleForObjects` :`Start` _returnvalue_2 :`End` (+ _returnvalue_2 (* (`KismetMathLibrary.GetForwardVector` (`SceneComponent.K2_GetComponentRotation` _transformcomponent)) 1000.0)) :`Radius` 150.0 :`ObjectTypes` (`|MakeArray` "ObjectTypeQuery3" :!type "EObjectTypeQuery Enum") :`DrawTime` 2.0))
        (if _returnvalue_3
          (bind (_bblockinghit _binitialoverlap _time _distance _location _impactpoint _normal _impactnormal _physmat _hitactor) (`GameplayStatics.BreakHitResult` _outhit))
          (cast `/Game/Characters/Horse/BP_Horse` _hitactor
            (:`CastFailed`
              ;;[0.05729 0.05729 0.05729 0.5] Target Lock On
              (set `self.Target Lock Actor` _hitactor)
              (set `self.isTargetLocked?` true)
              (set `CharacterMovementComponent.bOrientRotationToMovement` false _charactermovement_2)
              (set `CharacterMovementComponent.bUseControllerDesiredRotation` true _charactermovement_2)
              ;;[0.05729 0.05729 0.05729 0.5] Target Lock Widget
              (bind _returnvalue_4 (`|SpawnActorFromClass` "/Game/Player/BP_TargetLockWidget.BP_TargetLockWidget_C" (`KismetMathLibrary.MakeTransform` (`KismetMathLibrary.MakeVector` (.x (.location _returnvalue)) (.y (.location _returnvalue)) (+ (.z (.location _returnvalue)) 20.0)) (.rotation _returnvalue)) "AlwaysSpawn" "MultiplyWithRoot" null null))
              (bind _output_get (set `self.Target Lock Widget` _returnvalue_4))
              (`Actor.K2_AttachToActor` _output_get (`self.Target Lock Actor`) "None" "SnapToTarget" "SnapToTarget" "SnapToTarget" true))))))))

(event `self.ReceiveTick`
  (params (DeltaSeconds :type "Float (single-precision)"))
  (bind _charactermovement (`Character.CharacterMovement` (`self.Player BP`)))
  (bind (_returnvalue_roll _returnvalue_pitch _returnvalue_yaw) (`KismetMathLibrary.BreakRotator` (`KismetMathLibrary.FindLookAtRotation` (`Actor.K2_GetActorLocation` (`self.Player BP`)) (`Actor.K2_GetActorLocation` (`self.Target Lock Actor`)))))
  ;[0.05729 0.05729 0.05729 0.5] Target Lock
  ;;[0.05729 0.05729 0.05729 0.5] Target Lock Update
  (bind _target_lock_actor (`self.Target Lock Actor`)
    (:`then`
      (bind _asbp_enemy (cast `/Game/AI/BP_Enemy` _target_lock_actor))
      (if (`/Game/AI/BP_Enemy.isDead?` _asbp_enemy)
        ;;;[0.05729 0.05729 0.05729 0.5] Target Lock Off
        (set `self.isTargetLocked?` false)
        (set `self.movementDirection` "NewEnumerator0")
        (set `self.Target Lock Actor` null)
        (set `CharacterMovementComponent.bOrientRotationToMovement` true _charactermovement)
        (set `CharacterMovementComponent.bUseControllerDesiredRotation` false _charactermovement)
        (`Actor.K2_DestroyActor` (`self.Target Lock Widget`))
        (else
          (`Controller.SetControlRotation` (`Pawn.GetController` (`self.Player BP`)) (`KismetMathLibrary.MakeRotator` _returnvalue_roll (+ _returnvalue_pitch -20.0) _returnvalue_yaw)))))
    (:`else`)))

(event `EnhancedInput|/Game/Input/Actions/IA_LeftAttack`
  (params (ActionValue :type Boolean) (ElapsedSeconds :type "Float (double-precision)") (TriggeredSeconds :type "Float (double-precision)") (InputAction :type "InputAction Object Reference" :default "/Game/Input/Actions/IA_LeftAttack.IA_LeftAttack"))
  (bind _player_bp (`self.Player BP`))
  (bind _bpc_stats (`/Game/Player/BP_ThirdPersonCharacter.BPC_Stats` (`self.Player BP`)))
  ;[0.05729 0.05729 0.05729 0.5] Sword Combo Animation
  (:`Started`
    (if (and (not (`self.isAttacking?`)) (>= (`/Game/Player/BPC_Stats.stamina` (`/Game/Player/BP_ThirdPersonCharacter.BPC_Stats` _player_bp)) 10.0) (`/Game/Player/BP_ThirdPersonCharacter.weaponEquipped?` _player_bp))
      (set `self.isAttacking?` true)
      (`|PlayMontage` (`Character.Mesh` (`self.Player BP`)) "/Game/Characters/Mannequins/Anims/Attack/MM_DaggerAttackMontage.MM_DaggerAttackMontage"
        (:`then`
          (set `/Game/Player/BPC_Stats.regainStamina?` false _bpc_stats)
          (`/Game/Player/BPC_Stats.Increase Value` _bpc_stats "NewEnumerator1" -10.0 :!label _label))
        (:`OnCompleted`
          (set `self.isAttacking?` false :!label _label_2)
          (set `self.combo?` false)
          (set `/Game/Player/BPC_Stats.regainStamina?` true _bpc_stats))
        (:`OnInterrupted`
          (goto _label_2))
        (:`OnNotifyBegin`
          (if (and (`self.isAttacking?`) (`self.combo?`))
            (set `self.combo?` false)
            (goto _label)
            (else
              (`AnimInstance.Montage_Stop` (`SkeletalMeshComponent.GetAnimInstance` (`Character.Mesh` (`self.Player BP`))) 0.2 "/Game/Characters/Mannequins/Anims/Attack/MM_DaggerAttackMontage.MM_DaggerAttackMontage")))))
      (else
        (set `self.combo?` true)
        (`KismetSystemLibrary.PrintString` "cannot attack. missing weapon or stamina")))))

(event `End Damage Trace`
  ;[0.05729 0.05729 0.05729 0.5] Sword Traces
  (if (`KismetSystemLibrary.K2_IsValidTimerHandle` (stale `Begin Damage Trace` _returnvalue))
    (`KismetSystemLibrary.K2_ClearAndInvalidateTimerHandle` (stale `Begin Damage Trace` _returnvalue))))

(event `Begin Damage Trace`
  ;[0.05729 0.05729 0.05729 0.5] Sword Traces
  (bind _returnvalue (`KismetSystemLibrary.K2_SetTimerDelegate` (delegate `Damage Trace`) 0.01)))

(event `Damage Trace`
  (bind _player_bp (`self.Player BP`))
  (bind (_returnvalue_x _returnvalue_y _returnvalue_z) (`KismetMathLibrary.BreakVector` (`SceneComponent.K2_GetComponentLocation` (`/Game/Player/BP_ThirdPersonCharacter.Start Dagger Trace Pos` _player_bp))))
  ;[0.05729 0.05729 0.05729 0.5] Sword Traces
  (bind (_outhit _returnvalue) (`KismetSystemLibrary.SphereTraceSingleForObjects` :`Start` (`KismetMathLibrary.MakeVector` _returnvalue_x _returnvalue_y _returnvalue_z) :`End` (`SceneComponent.K2_GetComponentLocation` (`/Game/Player/BP_ThirdPersonCharacter.End Dagger Trace Pos` _player_bp)) :`Radius` 100.0 :`ObjectTypes` (`|MakeArray` "ObjectTypeQuery3" :!type "EObjectTypeQuery Enum") :`DrawDebugType` "ForDuration" :`DrawTime` 1.0))
  (if _returnvalue
    (`GameplayStatics.ApplyDamage` (`.HitActor` (`GameplayStatics.BreakHitResult` _outhit)) (`self.daggerDamage`))))

(event `EnhancedInput|/Game/Input/Actions/IA_Dodge`
  (params (ActionValue :type Boolean) (ElapsedSeconds :type "Float (double-precision)") (TriggeredSeconds :type "Float (double-precision)") (InputAction :type "InputAction Object Reference" :default "/Game/Input/Actions/IA_Dodge.IA_Dodge"))
  (bind _bpc_stats (`/Game/Player/BP_ThirdPersonCharacter.BPC_Stats` (`self.Player BP`)))
  ;[0.05729 0.05729 0.05729 0.5] Dodge
  (:`Started`
    (if (and (not (`self.isDodging?`)) (>= (`/Game/Player/BPC_Stats.stamina` (`/Game/Player/BP_ThirdPersonCharacter.BPC_Stats` (`self.Player BP`))) 25.0))
      (set `self.isDodging?` true)
      (`|ExecutionSequence`
        (:`then_0`
          (if (`CharacterMovementComponent.bUseControllerDesiredRotation` (`Character.CharacterMovement` (`self.Player BP`)))
            (if (`self.isTargetLocked?`)
              (switch `string` (`KismetTextLibrary.Conv_TextToString` (`KismetInputLibrary.Key_GetDisplayName` (`/Game/Player/BP_ThirdPersonCharacter.Direction Key` (`self.Player BP`))))
                (:`W`
                  (set `self.movementDirection` "NewEnumerator0" :!label _label_3))
                (:`A`
                  (set `self.movementDirection` "NewEnumerator1"))
                (:`S`
                  (set `self.movementDirection` "NewEnumerator2"))
                (:`D`
                  (set `self.movementDirection` "NewEnumerator3")))
              (else
                (goto _label_3)))))
        (:`then_1`
          (`|PlayMontage` (`Character.Mesh` (`self.Player BP`)) (select `/Game/Player/E_MovementDirection` (`self.movementDirection`) :`NewEnumerator0` "/Game/Characters/Mannequins/Anims/Dodge/Dodge_F_Montage.Dodge_F_Montage" :`NewEnumerator1` "/Game/Characters/Mannequins/Anims/Dodge/Dodge_L_Montage.Dodge_L_Montage" :`NewEnumerator2` "/Game/Characters/Mannequins/Anims/Dodge/Dodge_B_Montage.Dodge_B_Montage" :`NewEnumerator3` "/Game/Characters/Mannequins/Anims/Dodge/Dodge_R_Montage.Dodge_R_Montage" :!type "AnimMontage Object Reference") 0.9
            (:`then`
              (set `/Game/Player/BPC_Stats.regainStamina?` false _bpc_stats)
              (`/Game/Player/BPC_Stats.Increase Value` _bpc_stats "NewEnumerator1" -25.0))
            (:`OnCompleted`
              (set `self.isDodging?` false :!label _label_4)
              (set `/Game/Player/BPC_Stats.regainStamina?` true _bpc_stats))
            (:`OnInterrupted`
              (goto _label_4)))))
      (else
        (`KismetSystemLibrary.PrintString` "not enough stamina")))))