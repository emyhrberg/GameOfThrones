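; BP_WeaponPickable is a weapon pickup that an overlapping actor collects by touch.
; The construction script sets its static mesh from WeaponData.
; When PickupTrigger overlaps an actor implementing BPI_Interact, it passes WeaponData through PickupWeaponMessage, plays a pickup sound at its location and destroys itself.
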(event `self.PickupTrigger.OnComponentBeginOverlap`
  (params (OverlappedComponent :type "PrimitiveComponent Object Reference") (OtherActor :type "Actor Object Reference") (OtherComp :type "PrimitiveComponent Object Reference") (OtherBodyIndex :type Integer) (bFromSweep :type Boolean) (SweepResult :type "HitResult Structure (by ref)"))
  (if (`KismetSystemLibrary.DoesImplementInterface` OtherActor "/Game/Inventory/BPI_Interact.BPI_Interact_C")
    (message `/Game/Inventory/BPI_Interact.Pickup Weapon` OtherActor (`self.weaponData`))
    (`GameplayStatics.PlaySoundAtLocation` "/Engine/VREditor/Sounds/UI/Object_PickUp.Object_PickUp" (`self.K2_GetActorLocation`) (struct) 1.0 1.0 0.0 null null null null)
    (`self.K2_DestroyActor`)))

(fn `UserConstructionScript`
  (`StaticMeshComponent.SetStaticMesh` (`self.StaticMesh`) (`/Game/Inventory/BP_DA_Weapon.staticMesh` (`self.weaponData`))))